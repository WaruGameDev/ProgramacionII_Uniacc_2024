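; BP_Marble is the player-controlled marble, rolled and jumped with physics forces.
; On BeginPlay it registers the Enhanced Input mapping context; move input pushes the Ball scaled by SpeedBall, with Y inverted.
; Jump applies a mass-independent upward force only when a short, debug-drawn box trace below finds ground.
; Col overlaps send enter and exit messages to actors implementing BPI_Collision_Interface.
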(event OnComponentBeginOverlap(Col)
  (params (OverlappedComponent :type Primitive%20Component%20Object%20Reference) (OtherActor :type Actor%20Object%20Reference) (OtherComp :type Primitive%20Component%20Object%20Reference) (OtherBodyIndex :type Integer) (bFromSweep :type Boolean) (SweepResult :type Hit%20Result%20Structure%20%28by%20ref%29))
  ;[0.3214 0 1] Interface de colision
  (if (Utilities|DoesObjectImplementInterface OtherActor "/Game/BallAdventure/Blueprints/Interfaces/BPI_Collision_Interface.BPI_Collision_Interface_C")
    (Class|BPICollisionInterface|OnCollisionEnter(Message) OtherActor)))

(event OnComponentEndOverlap(Col)
  (params (OverlappedComponent :type Primitive%20Component%20Object%20Reference) (OtherActor :type Actor%20Object%20Reference) (OtherComp :type Primitive%20Component%20Object%20Reference) (OtherBodyIndex :type Integer))
  ;[0.3214 0 1] Interface de colision
  (if (Utilities|DoesObjectImplementInterface OtherActor "/Game/BallAdventure/Blueprints/Interfaces/BPI_Collision_Interface.BPI_Collision_Interface_C")
    (Class|BPICollisionInterface|OnCollisionExit(Message) OtherActor)))

(event Input|EnhancedActionEvents|EnhancedInputActionIA_Move
  (params (ActionValue :type Vector%202D%20Structure) (ElapsedSeconds :type Float%20%28double-precision%29) (TriggeredSeconds :type Float%20%28double-precision%29) (InputAction :type Input%20Action%20Object%20Reference :default "/Game/ThirdPerson/Input/Actions/IA_Move.IA_Move"))
  (bind _speedball (Variables|Default|GetSpeedBall))
  ;[0.4248 0 1] Movimiento de la pelota
  (Physics|AddForce (Variables|Default|GetBall) (Math|Vector|MakeVector (* (.x ActionValue) _speedball) (* (* (.y ActionValue) _speedball) -1.0) 0.0) "None" false))

(event Input|EnhancedActionEvents|EnhancedInputActionIA_Jump
  (params (ActionValue :type Boolean) (ElapsedSeconds :type Float%20%28double-precision%29) (TriggeredSeconds :type Float%20%28double-precision%29) (InputAction :type Input%20Action%20Object%20Reference :default "/Game/ThirdPerson/Input/Actions/IA_Jump.IA_Jump"))
  (bind _returnvalue (Transformation|GetActorLocation))
  ;[1 0.3517 0.6076] Salto
  (bind _returnvalue_2 (Collision|BoxTraceByChannel (+ _returnvalue "0.000000,0.000000,-50.000000") (+ _returnvalue "0.000000,0.000000,-60.000000") "45.000000,45.000000,0.100000" "0, 0, 0" "TraceTypeQuery1" false 0 "ForDuration" true "(R=1.000000,G=0.000000,B=0.000000,A=1.000000)" "(R=0.000000,G=1.000000,B=0.000000,A=1.000000)" 0.1))
  (if _returnvalue_2
    (Physics|AddForce (Variables|Default|GetBall) (Math|Vector|MakeVector 0.0 0.0 5e+04) "None" true)))

(event EventBeginPlay
  ;[0.86 0.1514 1] Obtener inputs
  (bind _asbp_marble_player_controller (Utilities|Casting|CastToBP_Marble_PlayerController (Pawn|GetController)))
  (Input|AddMappingContext (PlayerController|LocalPlayerSubsystems|GetEnhancedInputLocalPlayerSubsystem _asbp_marble_player_controller) "/Game/ThirdPerson/Input/IMC_Default.IMC_Default" 0 "(bIgnoreAllPressedKeysUntilRelease=True,bForceImmediately=False,bNotifyUserSettings=False)"))

(fn ConstructionScript)